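; Player-flown F-18 jet pawn with two switchable cameras, timeline-animated landing gear and breakable parts.
; Input axes feed the vehicle movement component, with smoothed throttle also scaling engine exhaust effects.
; A hit handler, whose binding is disconnected, breaks bone constraints; damage events hide thrusters or swap in a burning wreck.
; Tick spawns debug-key wing clouds and disables the mesh's autonomous-proxy physics replication at high speed.
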(event Custom|OnComponentHit_事件
  (params (HitComponent :type Primitive%20Component%20Object%20Reference) (OtherActor :type Actor%20Object%20Reference) (OtherComp :type Primitive%20Component%20Object%20Reference) (NormalImpulse :type Vector) (Hit :type Hit%20Result%20Structure%20%28by%20ref%29))
  (bind (_bblockinghit _binitialoverlap _time _distance _location _impactpoint _normal _impactnormal _physmat _hitactor _hitcomponent _hitbonename _bonename) (Collision|BreakHitResult Hit))
  (bind _returnvalue (Math|Vector|VectorLength NormalImpulse))
  (bind _mesh (Variables|Character|GetMesh))
  (bind _returnvalue_2 (== _bonename "rt_thruster_jnt"))
  (bind _returnvalue_3 (== _bonename "lf_thruster_jnt"))
  (if (> _returnvalue 5e+04)
    (Utilities|FlowControl|Sequence
      (:then_0
        (if (== _bonename "lf_slat_inner_jnt")
          (CallFunction|NewFunction _mesh NormalImpulse _impactpoint "lf_aileron_inner_jnt")))
      (:then_1
        (if (== _bonename "rt_slat_inner_jnt")
          (Class|SkeletalMeshComponent|BreakConstraint _mesh "0, 0, 0" "0, 0, 0" "rt_aileron_inner_jnt")
          (Class|MyWheeledVehiclePawn|Damaged "rt_aileron_inner_jnt")))
      (:then_2
        (if (or _returnvalue_2 _returnvalue_3)
          (if _returnvalue_2
            (Rendering|SetVisibility (Variables|Default|GetFX_Engine_01_F18C1) false false)
            (Class|MyWheeledVehiclePawn|Damaged _bonename :!label _label)
            (elif _returnvalue_3
              (Rendering|SetVisibility (Variables|Default|GetFX_Engine_01_F18C) false false)
              (goto _label)))
          (else
            (Class|SkeletalMeshComponent|BreakConstraint _mesh NormalImpulse _impactpoint _bonename)
            (goto _label))))
      (:then_3
        (if (and (== _bonename "cog_jnt") (> _returnvalue 5e+05))
          _)))))

(event Custom|Raised%20Gear
  (bind (_direction _gear _gear_doors) (Timeline|时间轴 PlayFromStart)
    (:Update
      (Variables|Default|SetGear _gear)
      (Variables|Default|SetGear%20Doors _gear_doors)
      (Variables|Default|SetGear%20Moving true))
    (:Finished
      (Variables|Default|SetCan%20Lower%20Gear? (== _gear_doors 1.0))
      (Variables|Default|SetGear%20Moving (Variables|Default|GetGear%20Moving)))))

(event Custom|Lower%20Gear
  (bind (_direction _gear _gear_doors) (Timeline|时间轴 ReverseFromEnd)
    (:Update
      (Variables|Default|SetGear _gear)
      (Variables|Default|SetGear%20Doors _gear_doors)
      (Variables|Default|SetGear%20Moving true))
    (:Finished
      (Variables|Default|SetCan%20Lower%20Gear? (== _gear_doors 1.0))
      (Variables|Default|SetGear%20Moving (Variables|Default|GetGear%20Moving)))))

(event EventBeginPlay)

(event Collision|EventActorBeginOverlap
  (params (OtherActor :type Actor%20Object%20Reference)))

(event EventAfterDisabelThruster
  (params (BoneName :type Name :default "None"))
  (if (== BoneName "rt_thruster_jnt")
    (Rendering|SetVisibility (Variables|Default|GetFX_Engine_01_F18C) false false)
    (else
      (Rendering|SetVisibility (Variables|Default|GetFX_Engine_01_F18C1) false false))))

(event Collision|EventHit
  (params (MyComp :type Primitive%20Component%20Object%20Reference) (Other :type Actor%20Object%20Reference) (OtherComp :type Primitive%20Component%20Object%20Reference) (bSelfMoved :type Boolean) (HitLocation :type Vector :default "0, 0, 0") (HitNormal :type Vector :default "0, 0, 0") (NormalImpulse :type Vector :default "0, 0, 0") (Hit :type Hit%20Result%20Structure%20%28by%20ref%29)))

(event EventAsyncPhysicsTick
  (params (DeltaSeconds :type Float%20%28single-precision%29) (SimSeconds :type Float%20%28single-precision%29))
  (if (> (Class|ChaosVehicleMovementComponent|GetForwardSpeedMPH (Variables|Default|GetVehicleMovementComponent)) 1e+02)
    _))

(event EventAfterExplode
  (bind _mesh (Variables|Character|GetMesh))
  (if (not (Variables|Default|GetExploded))
    (Effects|SpawnEmitterAttached "/Game/FXVarietyPack/Particles/P_ky_explosion.P_ky_explosion" (Variables|Character|GetMesh) "None" "0, 0, 0" "0, 0, 0" "5.000000,5.000000,5.000000" "KeepRelativeOffset" true "AutoRelease")
    (Variables|Default|SetExploded true)
    (Rendering|Material|SetMaterial (Variables|Character|GetMesh) 0 "/Game/VigilanteContent/Vehicles/West_Fighter_F18C/Damaged/Materials/M_West_Fighter_F18C_Damaged.M_West_Fighter_F18C_Damaged")
    (Rendering|SetVisibility (Variables|Default|GetFX_Wreckage_01_F18C) true false)
    (Rendering|SetVisibility (Variables|Default|GetFX_Engine_01_F18C) false false)
    (Rendering|SetVisibility (Variables|Default|GetFX_Engine_01_F18C1) false false)
    (Components|Activation|Deactivate (Variables|Default|GetVehicleMovementComponent))
    (Utilities|FlowControl|Delay 5.0)
    (Rendering|SetVisibility _mesh false false)
    (Components|SkinnedMesh|SetPhysicsAsset _mesh "/Game/VigilanteContent/Vehicles/West_Fighter_F18C/NewP.NewP" false)
    (Rendering|SetVisibility (Variables|Default|GetS_West_Fighter_F18C_Damaged) true false)))

(event EventTick
  (params (DeltaSeconds :type Float%20%28single-precision%29))
  (bind _mesh (Variables|Character|GetMesh))
  (Utilities|FlowControl|Sequence
    (:then_0
      (if (Variables|Default|Getcloud)
        (Effects|SpawnEmitteratLocation "/Game/FXVarietyPack/Particles/P_ky_cloud.P_ky_cloud" (Transformation|GetSocketLocation _mesh "cloudSocketRight") "0, 0, 0" "2.000000,2.000000,2.000000" true "AutoRelease")
        (Effects|SpawnEmitteratLocation "/Game/FXVarietyPack/Particles/P_ky_cloud.P_ky_cloud" (Transformation|GetSocketLocation _mesh "cloudSocketLeft") "0, 0, 0" "2.000000,2.000000,2.000000" true "AutoRelease")))
    (:then_1
      (if (> (Class|ChaosVehicleMovementComponent|GetForwardSpeedMPH (Variables|Default|GetVehicleMovementComponent)) 2e+02)
        (Variables|/Script/Engine.PrimitiveComponent|SetbReplicatePhysicsToAutonomousProxy (Variables|Character|GetMesh) false)
        (else
          (Variables|/Script/Engine.PrimitiveComponent|SetbReplicatePhysicsToAutonomousProxy (Variables|Character|GetMesh) true))))))

(event Input|AxisEvents|InputAxisMoveForward
  (params (AxisValue :type Float%20%28single-precision%29)))

(event Input|AxisEvents|InputAxisMoveForward/Backward
  (params (AxisValue :type Float%20%28single-precision%29))
  (bind _output_get (Variables|Default|SetElevator%20Pitch (Math|Interpolation|FInterpTo (stale _output_get) AxisValue (Utilities|Time|GetWorldDeltaSeconds) 0.9)))
  (Class|ChaosVehicleMovementComponent|SetPitchInput (Variables|Default|GetVehicleMovementComponent) AxisValue))

(event Input|AxisEvents|InputAxisMoveRight
  (params (AxisValue :type Float%20%28single-precision%29))
  (Class|ChaosVehicleMovementComponent|SetSteeringInput (Variables|Default|GetVehicleMovementComponent) AxisValue))

(event Input|AxisEvents|InputAxisMoveRight/Left
  (params (AxisValue :type Float%20%28single-precision%29))
  (Variables|Default|SetElevator%20Roll (Variables|Default|GetElevator%20Roll))
  (Class|ChaosVehicleMovementComponent|SetRollInput (Variables|Default|GetVehicleMovementComponent) AxisValue))

(event Input|AxisEvents|InputAxisYawControl
  (params (AxisValue :type Float%20%28single-precision%29))
  (Class|ChaosVehicleMovementComponent|SetYawInput (Variables|Default|GetVehicleMovementComponent) AxisValue))

(event Input|AxisEvents|InputAxisThrottleUp/Down
  (params (AxisValue :type Float%20%28single-precision%29))
  (bind _output_get (Variables|Default|SetThrust%20Value (Math|Interpolation|FInterpTo (stale _output_get) AxisValue (Utilities|Time|GetWorldDeltaSeconds) 1.0)))
  (Transformation|SetRelativeScale3D (Variables|Default|GetFX_Engine_01_F18C1) (Math|Vector|MakeVector (Math|Interpolation|FInterpTo _output_get AxisValue (Utilities|Time|GetWorldDeltaSeconds) 1.0) 1.0 1.0))
  (Transformation|SetRelativeScale3D (Variables|Default|GetFX_Engine_01_F18C) (Math|Vector|MakeVector (Math|Interpolation|FInterpTo _output_get AxisValue (Utilities|Time|GetWorldDeltaSeconds) 1.0) 1.0 1.0))
  (Class|ChaosVehicleMovementComponent|SetThrottleInput (Variables|Default|GetVehicleMovementComponent) (Math|Interpolation|FInterpTo _output_get AxisValue (Utilities|Time|GetWorldDeltaSeconds) 1.0)))

(event Input|AxisEvents|InputAxisRaiseGear
  (params (AxisValue :type Float%20%28single-precision%29))
  (if (and (> AxisValue 0.0) (not (Variables|Default|GetGear%20Moving)))
    (if (Variables|Default|GetCan%20Lower%20Gear?)
      (CallFunction|LowerGear)
      (else
        (CallFunction|RaisedGear)))))

(event Input|MouseEvents|MouseX
  (params (AxisValue :type Float%20%28single-precision%29))
  (Pawn|Input|AddControllerYawInput AxisValue))

(event Input|MouseEvents|MouseY
  (params (AxisValue :type Float%20%28single-precision%29))
  (Pawn|Input|AddControllerPitchInput (* AxisValue -1.0)))

(event Input|MouseEvents|DebugKeyRightMouseButton
  (params (Key :type Key%20Structure :default "None") (ActionValue :type Input%20Action%20Value%20Structure)))

(event Input|KeyboardEvents|DebugKeyTab
  (params (Key :type Key%20Structure :default "None") (ActionValue :type Input%20Action%20Value%20Structure))
  (:Pressed
    (Variables|Default|Setcloud true))
  (:Released
    (Variables|Default|Setcloud false)))

(event Input|MouseEvents|DebugKeyRightMouseButton
  (params (Key :type Key%20Structure :default "None") (ActionValue :type Input%20Action%20Value%20Structure))
  (bind _hit (Variables|Default|GetHit))
  (:Pressed
    (Class|MyWheeledVehiclePawn|ReceiveDamage "lf_slat_inner_jnt" 1e+02 "0.000000,0.000000,5000.000000" _hit)
    (Class|MyWheeledVehiclePawn|ReceiveDamage "rt_elevator_jnt" 1e+02 "0.000000,0.000000,5000.000000" _hit)
    (Class|MyWheeledVehiclePawn|ReceiveDamage "rt_thruster_jnt" 1e+02 "0.000000,0.000000,2000.000000" _hit)))

(event Input|KeyboardEvents|1
  (params (Key :type Key%20Structure :default "None"))
  (:Pressed
    (Components|Activation|Activate (Variables|Default|GetCamera) false)
    (Components|Activation|SetActive (Variables|Default|GetCamera1) false false)))

(event Input|KeyboardEvents|2
  (params (Key :type Key%20Structure :default "None"))
  (:Pressed
    (Components|Activation|SetActive (Variables|Default|GetCamera1) true false)
    (Components|Activation|SetActive (Variables|Default|GetCamera) false false)))

(fn ConstructionScript)

(fn NewFunction
  (params (self2 :type Skeletal%20Mesh%20Component%20Object%20Reference) (Impulse :type Vector) (HitLocation :type Vector) (BoneName :type Name))
  (Class|SkeletalMeshComponent|BreakConstraint self2 Impulse HitLocation BoneName)
  (Class|MyWheeledVehiclePawn|Damaged BoneName))

(fn HandleHit
  (params (BoneName :type Name)))