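; Boulder is a player-controlled rolling ball that delegates its motion to a RollingBallMovement component.
; Move axes feed throttle and steering, Space triggers a jump, and mouse input turns the controller's view with inverted pitch input.
; Each tick, the locally controlled instance passes control rotation to the component as travel direction.
; A debug key on V launches the Sphere upward with a velocity-change impulse.
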(event EventTick
  (params (DeltaSeconds :type Float%20%28single-precision%29))
  (if (Pawn|IsLocallyControlled)
    (Class|RollingBallMovementComponent|SetTravelDirectionInput (Variables|Default|GetRollingBallMovement) (Pawn|GetControlRotation :!class /Script/Engine.Pawn))))

(event Input|AxisEvents|InputAxisMoveForward
  (params (AxisValue :type Float%20%28single-precision%29))
  (Class|RollingBallMovementComponent|SetThrottleInput (Variables|Default|GetRollingBallMovement) AxisValue))

(event Input|AxisEvents|InputAxisMoveRight
  (params (AxisValue :type Float%20%28single-precision%29))
  (Class|RollingBallMovementComponent|SetSteeringInput (Variables|Default|GetRollingBallMovement) AxisValue))

(event Input|MouseEvents|MouseX
  (params (AxisValue :type Float%20%28single-precision%29))
  (Pawn|Input|AddControllerYawInput AxisValue))

(event Input|MouseEvents|MouseY
  (params (AxisValue :type Float%20%28single-precision%29))
  (Pawn|Input|AddControllerPitchInput (* AxisValue -1.0)))

(event Input|KeyboardEvents|DebugKeyV
  (params (Key :type Key%20Structure :default "None") (ActionValue :type Input%20Action%20Value%20Structure))
  (:Pressed
    (Physics|AddImpulse (Variables|Default|GetSphere) "0.000000,0.000000,600.000000" "None" true)))

(event Input|KeyboardEvents|SpaceBar
  (params (Key :type Key%20Structure :default "None"))
  (:Pressed
    (Class|RollingBallMovementComponent|Jump (Variables|Default|GetRollingBallMovement))))

(fn ConstructionScript)