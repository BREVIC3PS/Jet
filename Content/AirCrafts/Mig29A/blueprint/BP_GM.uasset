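; BP_GM, in the Mig29A aircraft folder, puts the local player in control of a BP_Pilot when play begins.
; BeginPlay gathers every PlayerStart into StartPoints and uses only the first entry.
; If that entry is valid, it destroys any pawn player 0 controls, spawns BP_Pilot at that transform, adjusting for collisions but always spawning, and possesses it.
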(event EventBeginPlay
  (bind _returnvalue (Game|GetPlayerController 0))
  (bind _startpoints (Variables|Default|GetstartPoints))
  (bind _returnvalue_2 (Pawn|GetControlledPawn _returnvalue))
  (bind _output (Utilities|Array|Get(acopy) _startpoints))
  (bind _outactors (Actor|GetAllActorsOfClass "/Script/Engine.PlayerStart"))
  (for _array_element _outactors
    (Utilities|Array|AddUnique (Variables|Default|GetstartPoints) _array_element))
  (Utilities|IsValid _output
    (:Is%20Valid
      (Utilities|IsValid _returnvalue_2
        (:Is%20Valid
          (Actor|DestroyActor _returnvalue_2))
        (:Is%20Not%20Valid
          _))
      (bind _returnvalue_3 (Game|SpawnActorfromClass "/Game/Aircraft/blueprint/BP_Pilot.BP_Pilot_C" (Transformation|GetActorTransform _output) "AdjustIfPossibleButAlwaysSpawn" 0 0))
      (Pawn|Possess _returnvalue _returnvalue_3))))

(fn ConstructionScript)