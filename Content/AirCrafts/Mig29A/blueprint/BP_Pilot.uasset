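; BP_Pilot is the player input blueprint for the MiG-29A aircraft, turning controls into flight state variables.
; Axis events set scaled Yaw, Pitch and Roll, while look axes drive controller pitch and yaw.
; SlowDown flips Acceleration negative while held and positive on release, and wheelOpen toggles the WheelOpen flag.
; It only records these values; no movement or gear logic runs in its graphs.
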(event Input|ActionEvents|InputActionwheelOpen
  (params (Key :type Key%20Structure :default "AnyKey"))
  ;[1 1 1] press G
  (:Pressed
    (if (Variables|Default|Getwheel_open)
      (Variables|Default|Setwheel_open false)
      (else
        (Variables|Default|Setwheel_open true)))))

(event Input|ActionEvents|InputActionSlowDown
  (params (Key :type Key%20Structure :default "AnyKey"))
  ;[1 1 1] press R
  (:Pressed
    (Variables|Default|Setacceleration -1e+02))
  (:Released
    (Variables|Default|Setacceleration 1e+02)))

(event Input|AxisEvents|InputAxisyawEvent
  (params (AxisValue :type Float%20%28single-precision%29))
  ;[1 1 1] press E and Q to control yaw
  (Variables|Default|Setyaw (* AxisValue 3e+01)))

(event Input|AxisEvents|InputAxispitchEvent
  (params (AxisValue :type Float%20%28single-precision%29))
  (Variables|Default|Setpitch (* AxisValue 3e+01)))

(event Input|AxisEvents|InputAxislookUp
  (params (AxisValue :type Float%20%28single-precision%29))
  (Pawn|Input|AddControllerPitchInput AxisValue))

(event Input|AxisEvents|InputAxislookRight
  (params (AxisValue :type Float%20%28single-precision%29))
  (Pawn|Input|AddControllerYawInput AxisValue))

(event Input|AxisEvents|InputAxisrollEvent
  (params (AxisValue :type Float%20%28single-precision%29))
  (Variables|Default|Setroll (* AxisValue 3e+01)))

(fn ConstructionScript)