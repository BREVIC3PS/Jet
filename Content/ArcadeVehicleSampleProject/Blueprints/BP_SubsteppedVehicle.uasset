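; BP_SubsteppedVehicle is a sample arcade vehicle with jump and reset controls, built on inherited vehicle logic.
; Space applies upward and random angular velocity impulses to CollisionMesh, and cuts lateral friction until released; R resets the vehicle.
; TraceFunc supplies the overridable trace as a complex Visibility line trace, leaving its HalfSize input unused.
; BeginPlay prints a hint for the debug-visuals console variable.
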(event EventBeginPlay
  (Development|PrintString "Use \"AV.DisplayDebugInfo 1\" for visuals." true true "(R=0.000000,G=0.660000,B=1.000000,A=1.000000)" 1e+01))

(event Input|KeyboardEvents|R
  (params (Key :type Key%20Structure :default "None"))
  (:Pressed
    (Class|AVBaseVehicle|ResetVehicle)))

(event Input|KeyboardEvents|SpaceBar
  (params (Key :type Key%20Structure :default "None"))
  (bind _collisionmesh (Variables|Default|GetCollisionMesh))
  (:Pressed
    (Physics|AddImpulse _collisionmesh (* (Transformation|GetActorUpVector) 5e+02) "None" true)
    (Class|PrimitiveComponent|AddAngularImpulseinDegrees _collisionmesh (Math|Vector|MakeVector (Math|Random|RandomFloatinRange -1e+02 1e+02) (Math|Random|RandomFloatinRange -1e+02 1e+02) 0.0) "None" true)
    (Variables|Default|SetLateralFrictionModifier 0.05))
  (:Released
    (Variables|Default|SetLateralFrictionModifier 1.0)))

(fn ConstructionScript)

(fn TraceFunc
  (params (Start :type Vector :default "0, 0, 0") (End :type Vector :default "0, 0, 0") (HalfSize :type Vector%202D%20Structure) (DrawDebugType :type EDrawDebugTrace%20Enum :default "None"))
  ;[1 1 1] The trace functionality can be overriden
  (bind (_outhit _returnvalue) (Collision|LineTraceByChannel Start End "TraceTypeQuery1" true 0 DrawDebugType))
  (return _outhit _returnvalue))